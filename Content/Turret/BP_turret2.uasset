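; Twin-barrel turret that tracks the first-person player character and fires bullets at it.
; On each PawnSensing sighting, the mesh eases toward the player in pitch and yaw while the actor follows in yaw.
; A FireRate Delay in the same event paces shots, spawning BP_bullet from alternating barrels.
; Collision overlap snaps the actor straight to face the player; a pitch clamp is left unused.
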(event OnSeePawn(PawnSensing)
  (params (Pawn :type Pawn%20Object%20Reference))
  (bind _asbp_fpcharacter (Utilities|Casting|CastToBP_FPcharacter Pawn))
  (Utilities|FlowControl|Sequence
    (:then_0
      (Transformation|SetWorldRotation (Variables|Default|GetStaticMesh) (Math|Rotator|MakeRotator 0.0 (.pitch (Math|Interpolation|RInterpTo (Transformation|GetActorRotation) (Math|Rotator|FindLookatRotation (Transformation|GetActorLocation) (Transformation|GetActorLocation _asbp_fpcharacter)) (Utilities|Time|GetWorldDeltaSeconds) (Math|Conversions|ToFloat(Integer) (Variables|Default|GetRotationSpeed)))) (.yaw (Math|Interpolation|RInterpTo (Transformation|GetActorRotation) (Math|Rotator|FindLookatRotation (Transformation|GetActorLocation) (Transformation|GetActorLocation _asbp_fpcharacter)) (Utilities|Time|GetWorldDeltaSeconds) (Math|Conversions|ToFloat(Integer) (Variables|Default|GetRotationSpeed))))) false false)
      (Transformation|SetActorRotation (Math|Rotator|MakeRotator 0.0 0.0 (.yaw (Math|Interpolation|RInterpTo (Transformation|GetActorRotation) (Math|Rotator|FindLookatRotation (Transformation|GetActorLocation) (Transformation|GetActorLocation _asbp_fpcharacter)) (Utilities|Time|GetWorldDeltaSeconds) (Math|Conversions|ToFloat(Integer) (Variables|Default|GetRotationSpeed)))))))
    (:then_1
      (Utilities|FlowControl|Delay (Variables|Default|GetFireRate))
      (if (== (Variables|Default|GetCurrentBarrelIndex) 0)
        (Game|SpawnActorfromClass "/Game/Blueprints/Turret/BP_bullet.BP_bullet_C" (Transformation|GetWorldTransform (Variables|Default|GetBarrel1)) "AlwaysSpawn" "MultiplyWithRoot" 0 0)
        (Variables|Default|SetCurrentBarrelIndex 1)
        (else
          (Game|SpawnActorfromClass "/Game/Blueprints/Turret/BP_bullet.BP_bullet_C" (Transformation|GetWorldTransform (Variables|Default|Getbarrel2)) "AlwaysSpawn" "MultiplyWithRoot" 0 0)
          (Variables|Default|SetCurrentBarrelIndex 0))))))

(event OnComponentBeginOverlap(collision)
  (params (OverlappedComponent :type Primitive%20Component%20Object%20Reference) (OtherActor :type Actor%20Object%20Reference) (OtherComp :type Primitive%20Component%20Object%20Reference) (OtherBodyIndex :type Integer) (bFromSweep :type Boolean) (SweepResult :type Hit%20Result%20Structure%20%28by%20ref%29))
  (bind _asbp_fpcharacter (Utilities|Casting|CastToBP_FPcharacter OtherActor))
  (Transformation|SetActorRotation (Math|Rotator|MakeRotator 0.0 (.pitch (Math|Rotator|FindLookatRotation (Transformation|GetActorLocation) (Transformation|GetActorLocation _asbp_fpcharacter))) (.yaw (Math|Rotator|FindLookatRotation (Transformation|GetActorLocation) (Transformation|GetActorLocation _asbp_fpcharacter))))))

(fn ConstructionScript)